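; Hexgrid Blueprint that procedurally builds a grid of static mesh tiles with varied heights.
; The construction script loops over GridX and GridY, placing tiles by the spacing values and shifting odd X columns along Y by Offset for a staggered hex layout.
; Each tile gets a random Z scale, re-rolled whenever construction runs, and is stored in WorldTiles.
; The event graph has no active logic.
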(event EventBeginPlay)

(event Collision|EventActorBeginOverlap
  (params (OtherActor :type Actor%20Object%20Reference)))

(event EventTick
  (params (DeltaSeconds :type Float%20%28single-precision%29)))

(fn ConstructionScript
  (for _index (range 0 (Variables|Default|GetGrid%20X))
    (for _index_2 (range 0 (Variables|Default|GetGrid%20Y))
      (bind _returnvalue (AddComponent|AddStaticMeshComponent false (Math|Transform|MakeTransform (Math|Vector|SelectVector (Math|Vector|MakeVector (* _index (Variables|Default|GetSpacing%20X)) (* _index_2 (Variables|Default|GetSpacing%20Y)) 0.0) (Math|Vector|MakeVector (* _index (Variables|Default|GetSpacing%20X)) (+ (* _index_2 (Variables|Default|GetSpacing%20Y)) (Variables|Default|GetOffset)) 0.0) (== (Math|Integer|%(Integer) _index 2) 0)) "0, 0, 0" "1,1,1")))
      (Transformation|SetWorldScale3D _returnvalue (Math|Vector|MakeVector 1.0 1.0 (Math|Random|RandomFloatinRange 1.0 5.0)))
      (Utilities|Array|Add (Variables|Default|GetWorld%20tiles) _returnvalue))))