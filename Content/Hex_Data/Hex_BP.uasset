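; Hex tile actor for a world grid, with a random height, hover highlight and click readout.
; The construction script adds an entry to WorldGrid, then sets the root's Z scale and the Height variable from separate random rolls, so the two values can differ.
; Cursor-over events toggle the Mouse_Hover scalar material parameter on the mesh, and clicking prints Height.
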(event OnBeginCursorOver(Hex_mesh)
  (params (TouchedComponent :type Primitive%20Component%20Object%20Reference))
  (Rendering|Material|SetScalarParameterValueonMaterials (Variables|Default|GetHex_mesh) "Mouse_Hover" 1.0))

(event OnEndCursorOver(Hex_mesh)
  (params (TouchedComponent :type Primitive%20Component%20Object%20Reference))
  (Rendering|Material|SetScalarParameterValueonMaterials (Variables|Default|GetHex_mesh) "Mouse_Hover" 0.0))

(event MouseInput|EventActorOnClicked
  (params (ButtonPressed :type Key%20Structure :default "None"))
  (Development|PrintString (Utilities|String|ToString(Float) (Variables|Default|GetHeight))))

(fn ConstructionScript
  (bind _returnvalue (Math|Random|RandomFloatinRange 1.0 5.0))
  (Utilities|Array|Add (Variables|Default|GetWorld%20Grid) 0)
  (Transformation|SetWorldScale3D (Variables|Transformation|GetRootComponent) (Math|Vector|MakeVector 1.0 1.0 _returnvalue))
  (Variables|Default|SetHeight _returnvalue))