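; Game mode Blueprint with logic for generating a hex grid, though the generation loop has no connected entry point and never runs.
; The loop spawns Hex_BP actors in columns, offsetting odd columns on Y for staggering, and adds them to HexGrid.
; It also copies the grid dimensions to GameState_BP on every iteration.
; Hex_Created_Event prints a debug string and assigns the last added array index as the newest hex's HexID.
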(event Custom|Hex_Created_Event
  (Development|PrintString "Poopy")
  (Variables|/Game/Hex_Data/Hex_BP.Hex_BP_C|SetHex_ID (stale _returnvalue) (stale _returnvalue)))

(fn ConstructionScript)

(fn SendGridXandY
  (bind _returnvalue (Game|GetGameState))
  (bind _asgame_state_bp (Utilities|Casting|CastToGameState_BP _returnvalue))
  (Variables|/Game/StarterContent/Maps/GameState_BP.GameState_BP_C|SetGrid%20X _asgame_state_bp (Variables|Default|GetGrid%20X))
  (bind _asgame_state_bp_2 (Utilities|Casting|CastToGameState_BP _returnvalue))
  (Variables|/Game/StarterContent/Maps/GameState_BP.GameState_BP_C|SetGrid%20Y _asgame_state_bp_2 (Variables|Default|GetGrid%20Y))
  (return))